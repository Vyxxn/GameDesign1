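; BP_UIPickup is a Blueprint that displays a WidgetUI instance through its Widget component.
; BeginPlay creates the widget and assigns it to that component.
; RotateToPlayer turns the component toward the first player's camera manager location with a look-at rotation, re-calling itself every 0.1 seconds through a Delay instead of Tick.
; Nothing in this file starts that loop, and no pickup logic is present.
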(event Custom|Rotate%20To%20Player
  (Transformation|SetWorldRotation (Variables|Default|GetWidget) (Math|Rotator|FindLookatRotation (Transformation|GetWorldLocation (Variables|Default|GetWidget)) (Transformation|GetWorldLocation (Variables|/Script/Engine.Actor|GetRootComponent (Game|GetPlayerCameraManager 0)))) false false)
  (Utilities|FlowControl|Delay 0.1)
  (CallFunction|RotatetoPlayer))

(event EventBeginPlay
  (bind _returnvalue (UserInterface|CreateWidget "/Game/Widgets/WidgetUI.WidgetUI_C"))
  (UserInterface|SetWidget (Variables|Default|GetWidget) _returnvalue) ; How do I reference WidgetUI through here?
)

(event Collision|EventActorBeginOverlap
  (params (OtherActor :type Actor%20Object%20Reference)))

(event EventTick
  (params (DeltaSeconds :type Float%20%28single-precision%29)))

(fn ConstructionScript)